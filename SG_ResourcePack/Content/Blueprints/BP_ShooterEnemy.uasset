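; Enemy that alternates between moving to random points around the player and firing bullet bursts, turning to face the player throughout.
; Tick moves it at constant speed to a random 3D offset from the player's position, then triggers Shoot through a resettable DoOnce.
; Shoot repeats on a short delay, firing three muzzles, one at the player and two at random nearby points.
; After MaxShots volleys, it picks a new destination.
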(event Custom|Shoot
  (bind _returnvalue (Game|Player|GetPlayerPawn 0))
  (bind _returnvalue_2 (Game|Player|GetPlayerPawn 0))
  (bind _returnvalue_3 (Transformation|GetActorLocation _returnvalue_2))
  (bind _returnvalue_4 (Math|Random|RandomPointinBoundingBox _returnvalue_3 "500.000000,500.000000,500.000000"))
  (if (>= (Variables|Default|GetCurrent%20Shot) (Variables|Default|GetMax%20Shots))
    (Variables|Default|SetCurrent%20Shot 0)
    (CallFunction|SelectMoveLocation)
    (else
      (Math|Integer|IncrementInt (Variables|Default|GetCurrent%20Shot)
        (:%20%20
          (Utilities|IsValid (Game|Player|GetPlayerPawn 0)
            (:Is%20Valid
              (Utilities|FlowControl|Sequence
                (:then_0
                  (Utilities|IsValid _returnvalue
                    (:Is%20Valid
                      (CallFunction|ShootBullet (Variables|Default|GetMuzzle%201) (Transformation|GetActorLocation _returnvalue)))))
                (:then_1
                  (CallFunction|ShootBullet (Variables|Default|GetMuzzle%202) _returnvalue_4))
                (:then_2
                  (CallFunction|ShootBullet (Variables|Default|GetMuzzle%203) _returnvalue_4))
                (:then_3
                  (Utilities|FlowControl|Delay 0.2)
                  (CallFunction|Shoot))))))))))

(event Custom|ResetShoot
  (Utilities|FlowControl|DoOnce false) ; enters at Reset
)

(event EventBeginPlay
  (|CallParentFunction)
  (CallFunction|SelectMoveLocation))

(event EventTick
  (params (DeltaSeconds :type Float%20%28single-precision%29))
  (CallFunction|RotateTowardsPlayer (Game|GetPlayerController 0) self DeltaSeconds 5.0)
  (if (Variables|Default|GetMoving)
    (Transformation|SetActorLocation (Math|Interpolation|VInterptoConstant (Transformation|GetActorLocation) (Variables|Default|GetTarget%20Location) (Utilities|Time|GetWorldDeltaSeconds) (Math|Conversions|ToFloat(Integer) (Variables|Default|GetSpeed))) false false)
    (if (Utilities|Operators|EqualEqual (Transformation|GetActorLocation) (Variables|Default|GetTarget%20Location) 1e+01)
      (Variables|Default|SetMoving false)
      (Utilities|FlowControl|DoOnce false
        (:Completed
          (CallFunction|Shoot))))))

(fn ConstructionScript
  (|CallParentFunction))

(fn SelectMoveLocation
  (bind _returnvalue (Game|Player|GetPlayerPawn 0))
  (CallFunction|ResetShoot)
  (Utilities|IsValid _returnvalue
    (:Is%20Valid
      (Variables|Default|SetTarget%20Location (+ (Transformation|GetActorLocation _returnvalue) (* (Math|Random|RandomUnitVector) (Math|Random|RandomIntegerinRange 5000 8500))))
      (Variables|Default|SetMoving true))))

(fn ShootBullet
  (params (From :type Scene%20Component%20Object%20Reference) (Target :type Vector%20%28by%20ref%29))
  (bind _returnvalue (Transformation|GetWorldLocation From))
  (bind _returnvalue_2 (Game|SpawnActorfromClass "/Game/Blueprints/BP_EnemyBullet.BP_EnemyBullet_C" (Math|Transform|MakeTransform _returnvalue "0, 0, 0" "1.000000,1.000000,1.000000") "Undefined" "MultiplyWithRoot" 0 0))
  (Default|BulletonSpawn _returnvalue_2 (Math|Vector|GetForwardVector (Math|Rotator|FindLookatRotation _returnvalue Target))))