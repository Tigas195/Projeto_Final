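; Missile actor that seeks actors tagged Enemy and explodes on reaching one, applying area damage.
; A valid enemy target passed at launch is chased each Tick by constant-speed location interpolation.
; Without one, or if it becomes invalid, HomingDetectorCollision overlaps can acquire an enemy for ProjectileMovement homing, gated by DoOnce nodes.
; ExplodeDetection triggers damage to enemies inside DamageArea, then spawns an explosion and destroys the missile.
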(event OnComponentBeginOverlap(HomingDetectorCollision)
  (params (OverlappedComponent :type Primitive%20Component%20Object%20Reference) (OtherActor :type Actor%20Object%20Reference) (OtherComp :type Primitive%20Component%20Object%20Reference) (OtherBodyIndex :type Integer) (bFromSweep :type Boolean) (SweepResult :type Hit%20Result%20Structure%20%28by%20ref%29))
  (if (Actor|ActorHasTag OtherActor "Enemy")
    (Utilities|FlowControl|DoOnce (Variables|Default|GetCustom%20Homing)
      (:Completed
        (CallFunction|ResetSearchforTarget)
        (Variables|Default|SetTarget OtherActor)
        (CallFunction|SetHoming)))))

(event OnComponentBeginOverlap(ExplodeDetection)
  (params (OverlappedComponent :type Primitive%20Component%20Object%20Reference) (OtherActor :type Actor%20Object%20Reference) (OtherComp :type Primitive%20Component%20Object%20Reference) (OtherBodyIndex :type Integer) (bFromSweep :type Boolean) (SweepResult :type Hit%20Result%20Structure%20%28by%20ref%29))
  (if (Actor|ActorHasTag OtherActor "Enemy")
    (Utilities|FlowControl|DoOnce false
      (:Completed
        (CallFunction|ApplyAOEDamage)))))

(event Custom|Reset%20Colision
  (Utilities|FlowControl|DoOnce (Variables|Default|GetCustom%20Homing)) ; enters at Reset
)

(event Custom|Reset%20Search%20for%20target
  (Utilities|FlowControl|DoOnce false) ; enters at Reset
)

(event Custom|Lauch%20Missile
  (params (Velocity :type Vector) (Target%20Actor :type Actor%20Object%20Reference))
  (Variables|Default|SetTarget%20Velocity Velocity)
  (bind _output_get (Variables|Default|SetTarget Target%20Actor))
  (Utilities|IsValid _output_get
    (:Is%20Valid
      (if (Actor|ActorHasTag (Variables|Default|GetTarget) "Enemy")
        (Variables|Default|SetCustom%20Homing true)
        (else
          (Variables|/Script/Engine.MovementComponent|SetVelocity (Variables|Default|GetProjectileMovement) (* (Variables|Default|GetTarget%20Velocity) 20000) :!label _label)
          (Variables|/Script/Engine.PrimitiveComponent|SetbGenerateOverlapEvents (Variables|Default|GetHoming%20Detector%20Collision) true))))
    (:Is%20Not%20Valid
      (goto _label))))

(event EventBeginPlay)

(event Collision|EventActorBeginOverlap
  (params (OtherActor :type Actor%20Object%20Reference)))

(event EventTick
  (params (DeltaSeconds :type Float%20%28single-precision%29))
  (if (Variables|Default|GetCustom%20Homing)
    (Utilities|IsValid (Variables|Default|GetTarget)
      (:Is%20Valid
        (Transformation|SetActorLocation (Math|Interpolation|VInterptoConstant (Transformation|GetActorLocation) (Transformation|GetActorLocation (Variables|Default|GetTarget)) DeltaSeconds 5e+04) false false))
      (:Is%20Not%20Valid
        (Utilities|FlowControl|DoOnce false
          (:Completed
            (Variables|Default|SetCustom%20Homing false)
            (Variables|/Script/Engine.PrimitiveComponent|SetbGenerateOverlapEvents (Variables|Default|GetHoming%20Detector%20Collision) true)
            (CallFunction|ResetColision)))))))

(fn ConstructionScript)

(fn ApplyAOEDamage
  (for _array_element (Collision|GetOverlappingActors (Variables|Default|GetDamage%20Area) 0 :!class /Script/Engine.PrimitiveComponent)
    (if (Actor|ActorHasTag _array_element "Enemy")
      (Game|Damage|ApplyDamage _array_element 1e+01 0 0)))
  (CallFunction|Death))

(fn SetHoming
  (bind _projectilemovement (Variables|Default|GetProjectileMovement))
  (Variables|/Script/Engine.MovementComponent|SetVelocity _projectilemovement "0, 0, 0")
  (Variables|/Script/Engine.ProjectileMovementComponent|SetbIsHomingProjectile _projectilemovement true)
  (Variables|/Script/Engine.ProjectileMovementComponent|SetHomingTargetComponent _projectilemovement (Actor|GetComponentbyClass (Variables|Default|GetTarget) "/Script/Engine.SceneComponent")))

(fn Death
  (Effects|SpawnEmitteratLocation "/Game/StarterContent/Particles/P_Explosion.P_Explosion" (Transformation|GetActorLocation) "0, 0, 0" "20.000000,20.000000,20.000000")
  (Actor|DestroyActor))