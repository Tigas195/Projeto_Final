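; BP_BoomEnemy is an enemy actor that homes in on the player pawn.
; Each tick it turns toward the player through RotateTowardsPlayer and moves at constant Speed with VInterpToConstant, without sweep, so movement ignores blocking collision.
; On BeginPlay it binds a RotatingMovement component to EnemyBody, so the body spins independently of the actor's facing.
; The graph contains no explosion or damage logic.
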(event EventBeginPlay
  (Components|Movement|SetUpdatedComponent (Variables|Default|GetRotatingMovement) (Variables|Default|GetEnemyBody)))

(event EventTick
  (params (DeltaSeconds :type Float%20%28single-precision%29))
  (bind _returnvalue (Game|Player|GetPlayerPawn 0))
  (CallFunction|RotateTowardsPlayer (Game|GetPlayerController 0) self DeltaSeconds 1e+01)
  (Utilities|IsValid _returnvalue
    (:Is%20Valid
      (Transformation|SetActorLocation (Math|Interpolation|VInterptoConstant (Transformation|GetActorLocation) (Transformation|GetActorLocation _returnvalue) DeltaSeconds (Math|Conversions|ToFloat(Integer) (Variables|Default|GetSpeed))) false false))))

(fn ConstructionScript
  (|CallParentFunction))