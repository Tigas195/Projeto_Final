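; GM_SpaceGame is the game mode for a space game, handling the main menu and player ship spawning.
; On BeginPlay it creates the WG_MainMenu widget, stores a reference and shows it with the mouse cursor and UI-only input.
; Separate events hide the menu to restore game-only input, and spawn a BP_PlayerSpaceship, with neither called within this graph.
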(event Custom|Show%20main%20menu
  (bind _returnvalue (Game|GetPlayerController 0))
  (bind _wg_mainmenu_ref (Variables|Default|GetWG_MainMenu_Ref))
  (Variables|/Script/Engine.PlayerController|SetbShowMouseCursor _returnvalue true)
  (Input|SetInputModeUIOnly _returnvalue _wg_mainmenu_ref "DoNotLock" false)
  (UserInterface|Viewport|AddtoViewport _wg_mainmenu_ref 0))

(event Custom|Hide%20Main%20Menu
  (bind _returnvalue (Game|GetPlayerController 0))
  (Variables|/Script/Engine.PlayerController|SetbShowMouseCursor _returnvalue false)
  (Input|SetInputModeGameOnly _returnvalue false)
  (Widget|RemovefromParent (Variables|Default|GetWG_MainMenu_Ref)))

(event Custom|Spaw%20Player
  (Game|SpawnActorfromClass "/Game/Blueprints/BP_PlayerSpaceship.BP_PlayerSpaceship_C" (Math|Transform|MakeTransform "0, 0, 0" "0, 0, 0" "1.000000,1.000000,1.000000") "Undefined" "MultiplyWithRoot" 0 0))

(event EventBeginPlay
  (bind _returnvalue (UserInterface|CreateWidget "/Game/UI/WG_MainMenu.WG_MainMenu_C" (Game|GetPlayerController 0)))
  (Variables|Default|SetWG_MainMenu_Ref _returnvalue)
  (CallFunction|ShowMainMenu))

(fn ConstructionScript)