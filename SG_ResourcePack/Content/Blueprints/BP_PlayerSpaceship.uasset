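; Player spaceship pawn with six-direction flight, mouse look and stamina-limited sprinting.
; Tick turns held-key flags into input for FloatingPawnMovement, banks the body when strafing and shows Niagara trails while moving.
; Sprint raises max speed and plays a reversible timeline scaling thrusters and widening FOV.
; A looping timer drains or regenerates stamina, updates the gameplay widget, stops sprint when empty and pauses when full.
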(event Custom|Stop%20Sprint%20Effect
  (bind _sprint_alpha (Timeline|TL_Sprint Reverse)
    (:Update
      (Transformation|SetWorldScale3D (Variables|Default|GetP_Thruster) (Math|Vector|Lerp(Vector) "0.250000,0.500000,0.500000" "0.500000,0.500000,1.500000" _sprint_alpha))
      (Camera|SetFieldOfView (Variables|Default|GetCamera) (Math|Float|Lerp 9e+01 1.1e+02 _sprint_alpha)))))

(event Custom|Start%20Timers
  (bind _returnvalue (Utilities|Time|SetTimerbyEvent (delegate Custom|Stamina%20Regen) 1.0 true))
  (Variables|Default|SetStamina%20Timer%20Handle _returnvalue))

(event Custom|Stamina%20Regen
  (bind _max_stamina (Variables|Movement|GetMax%20Stamina))
  (bind _output_get (Variables|Movement|SetCurrent%20Stamina (Math|Float|Clamp(Float) (Math|Float|SelectFloat (- (Variables|Movement|GetCurrent%20Stamina) (Variables|Default|GetStamina%20Consumption%20Value)) (+ (Variables|Movement|GetCurrent%20Stamina) (Variables|Default|GetStamina%20Regen%20Value)) (Variables|Movement|GetIs%20Sprinting)) 0.0 _max_stamina)))
  (Default|UpdateStaminaPercent (Variables|Default|GetWG%20Gameplay%20Ref) (/ _output_get _max_stamina))
  (Utilities|FlowControl|Sequence
    (:then_0
      (if (== (Variables|Movement|GetCurrent%20Stamina) 0.0)
        (CallFunction|StopSprinting)))
    (:then_1
      (if (== (Variables|Movement|GetCurrent%20Stamina) (Variables|Movement|GetMax%20Stamina))
        (Utilities|Time|PauseTimerbyHandle (Variables|Default|GetStamina%20Timer%20Handle))))))

(event Custom|Start%20Sprint%20Effect
  (bind _sprint_alpha (Timeline|TL_Sprint Play)
    (:Update
      (Transformation|SetWorldScale3D (Variables|Default|GetP_Thruster) (Math|Vector|Lerp(Vector) "0.250000,0.500000,0.500000" "0.500000,0.500000,1.500000" _sprint_alpha))
      (Camera|SetFieldOfView (Variables|Default|GetCamera) (Math|Float|Lerp 9e+01 1.1e+02 _sprint_alpha)))))

(event EventBeginPlay
  (Pawn|Possess (Game|GetPlayerController 0) self)
  (CallFunction|SetDefaults)
  (Utilities|FlowControl|Sequence
    (:then_0
      ;[0.15 0.15 0.15 0.5] Criar Widget Gameplay
      (bind _returnvalue (UserInterface|CreateWidget "/Game/UI/WG_Gameplay.WG_Gameplay_C" (Game|GetPlayerController 0)))
      (bind _output_get (Variables|Default|SetWG%20Gameplay%20Ref _returnvalue))
      (UserInterface|Viewport|AddtoViewport _output_get 0)
      (Default|UpdateStaminaPercent (Variables|Default|GetWG%20Gameplay%20Ref) (/ (Variables|Movement|GetCurrent%20Stamina) (Variables|Movement|GetMax%20Stamina))))
    (:then_1
      (CallFunction|StartTimers))))

(event Collision|EventActorBeginOverlap
  (params (OtherActor :type Actor%20Object%20Reference)))

(event EventTick
  (params (DeltaSeconds :type Float%20%28single-precision%29))
  (Utilities|FlowControl|Sequence
    (:then_0
      (Class|PawnMovementComponent|AddInputVector (Variables|Default|GetFloatingPawnMovement) (CallFunction|MovementMath) false))
    (:then_1
      (CallFunction|RotateShipwhenStrafe)
      (Rendering|SetVisibility (Variables|Default|GetNS_Trail%20L) (not (Utilities|Operators|EqualEqual :A (Transformation|GetVelocity))) false))))

(event Input|MouseEvents|MouseX
  (params (AxisValue :type Float%20%28single-precision%29))
  (Pawn|Input|AddControllerYawInput (* AxisValue 0.5)))

(event Input|MouseEvents|MouseY
  (params (AxisValue :type Float%20%28single-precision%29))
  (Pawn|Input|AddControllerPitchInput (* (* AxisValue -1.0) 0.5)))

(event Input|KeyboardEvents|W
  (params (Key :type Key%20Structure))
  ;[0.15 0.15 0.15 0.5] Setting Input Status
  (:Pressed
    (Variables|Inputs|SetW%20is%20Pressed true))
  (:Released
    (Variables|Inputs|SetW%20is%20Pressed false)))

(event Input|KeyboardEvents|S
  (params (Key :type Key%20Structure))
  ;[0.15 0.15 0.15 0.5] Setting Input Status
  (:Pressed
    (Variables|Inputs|SetS%20is%20Pressed true))
  (:Released
    (Variables|Inputs|SetS%20is%20Pressed false)))

(event Input|KeyboardEvents|A
  (params (Key :type Key%20Structure))
  ;[0.15 0.15 0.15 0.5] Setting Input Status
  (:Pressed
    (Variables|Inputs|SetA%20is%20Pressed true))
  (:Released
    (Variables|Inputs|SetA%20is%20Pressed false)))

(event Input|KeyboardEvents|D
  (params (Key :type Key%20Structure))
  ;[0.15 0.15 0.15 0.5] Setting Input Status
  (:Pressed
    (Variables|Inputs|SetD%20is%20Pressed true))
  (:Released
    (Variables|Inputs|SetD%20is%20Pressed false)))

(event Input|KeyboardEvents|SpaceBar
  (params (Key :type Key%20Structure))
  ;[0.15 0.15 0.15 0.5] Setting Input Status
  (:Pressed
    (Variables|Inputs|SetSpace%20is%20Pressed true))
  (:Released
    (Variables|Inputs|SetSpace%20is%20Pressed false)))

(event Input|KeyboardEvents|LeftCtrl
  (params (Key :type Key%20Structure))
  ;[0.15 0.15 0.15 0.5] Setting Input Status
  (:Pressed
    (Variables|Inputs|SetLeft%20Ctrl%20is%20Pressed true))
  (:Released
    (Variables|Inputs|SetLeft%20Ctrl%20is%20Pressed false)))

(event Input|KeyboardEvents|LeftShift
  (params (Key :type Key%20Structure))
  ;[0.15 0.15 0.15 0.5] Setting Input Status
  (:Pressed
    (Variables|Movement|SetIs%20Sprinting true)
    (Variables|/Script/Engine.FloatingPawnMovement|SetMaxSpeed (Variables|Default|GetFloatingPawnMovement) 2.5e+03)
    (Utilities|Time|UnpauseTimerbyHandle (Variables|Default|GetStamina%20Timer%20Handle))
    (CallFunction|StartSprintEffect))
  (:Released
    (CallFunction|StopSprinting)))

(fn ConstructionScript)

(fn MovementMath
  (bind _returnvalue (Transformation|GetActorRightVector))
  (bind _returnvalue_2 (Transformation|GetActorUpVector))
  (bind _returnvalue_3 (Transformation|GetActorForwardVector))
  (Variables|Movement|SetDirection%20FB (select (or (and (Variables|Inputs|GetW%20is%20Pressed) (Variables|Inputs|GetS%20is%20Pressed)) (and (not (Variables|Inputs|GetW%20is%20Pressed)) (not (Variables|Inputs|GetS%20is%20Pressed)))) "0, 0, 0" (Math|Vector|SelectVector (* _returnvalue_3 -1) _returnvalue_3 (Variables|Inputs|GetS%20is%20Pressed))))
  (Variables|Movement|SetDirection%20LR (select (or (and (Variables|Inputs|GetA%20is%20Pressed) (Variables|Inputs|GetD%20is%20Pressed)) (and (not (Variables|Inputs|GetD%20is%20Pressed)) (not (Variables|Inputs|GetA%20is%20Pressed)))) "0, 0, 0" (Math|Vector|SelectVector (* _returnvalue -1) _returnvalue (Variables|Inputs|GetA%20is%20Pressed))))
  (Variables|Movement|SetDirection%20UD (select (or (and (Variables|Inputs|GetSpace%20is%20Pressed) (Variables|Inputs|GetLeft%20Ctrl%20is%20Pressed)) (and (not (Variables|Inputs|GetSpace%20is%20Pressed)) (not (Variables|Inputs|GetLeft%20Ctrl%20is%20Pressed)))) "0, 0, 0" (Math|Vector|SelectVector (* _returnvalue_2 -1) _returnvalue_2 (Variables|Inputs|GetLeft%20Ctrl%20is%20Pressed))))
  (return (+ (Variables|Movement|GetDirection%20FB) (Variables|Movement|GetDirection%20LR) (Variables|Movement|GetDirection%20UD))))

(fn RotateShipwhenStrafe
  (bind _body (Variables|Default|GetBody))
  (bind _original_body_relative_rotation (Variables|Default|GetOriginal%20Body%20Relative%20Rotation))
  (bind _body_2 (Variables|Default|GetBody))
  (if (or (and (Variables|Inputs|GetA%20is%20Pressed) (Variables|Inputs|GetD%20is%20Pressed)) (and (not (Variables|Inputs|GetD%20is%20Pressed)) (not (Variables|Inputs|GetA%20is%20Pressed))))
    (Transformation|SetRelativeRotation _body_2 (Math|Interpolation|RInterpTo (Variables|/Script/Engine.SceneComponent|GetRelativeRotation _body_2) (Variables|Default|GetOriginal%20Body%20Relative%20Rotation) (Utilities|Time|GetWorldDeltaSeconds) 1.0) false false)
    (else
      (Transformation|SetRelativeRotation _body (Math|Interpolation|RInterpTo (Variables|/Script/Engine.SceneComponent|GetRelativeRotation _body) (Math|Rotator|CombineRotators (Variables|Default|GetOriginal%20Body%20Relative%20Rotation) (Math|Rotator|SelectRotator (Math|Rotator|CombineRotators _original_body_relative_rotation "0.000000,0.000000,-15.000000") (Math|Rotator|CombineRotators _original_body_relative_rotation "0.000000,0.000000,15.000000") (Variables|Inputs|GetA%20is%20Pressed))) (Utilities|Time|GetWorldDeltaSeconds) 1.0) false false))))

(fn SetDefaults
  (Variables|Default|SetOriginal%20Body%20Relative%20Rotation (Variables|/Script/Engine.SceneComponent|GetRelativeRotation (Variables|Default|GetBody)))
  (Variables|Movement|SetCurrent%20Stamina (Variables|Movement|GetMax%20Stamina)))

(fn StopSprinting
  (Variables|Movement|SetIs%20Sprinting false)
  (Variables|/Script/Engine.FloatingPawnMovement|SetMaxSpeed (Variables|Default|GetFloatingPawnMovement) 1.2e+03)
  (CallFunction|StopSprintEffect))